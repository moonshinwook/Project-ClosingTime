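; Player character Blueprint that handles roll, crouch and assassination actions.
; Roll plays a montage and crouch input toggles crouching, both gated by CanProcessActionInput.
; When BeginAssassionation succeeds, assassination input motion-warps the player to the BP_MyEnemy's AssassinationPoint and plays the kill montage while the enemy plays its choke.
; EndAssassionation runs when the montage completes or is interrupted.
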(event Custom|Try%20Roll
  ;[0.15 0.15 0.15 0.5] TryRoll
  (if (Class|MyPlayer|CanProcessActionInput)
    (Animation|PlayAnimMontage "/Game/Animations/Montages/AM_Roll_front.AM_Roll_front" 1.0 "None")))

(event Input|EnhancedActionEvents|EnhancedInputActionIA_Crouch
  (params (ActionValue :type Boolean) (ElapsedSeconds :type Float%20%28double-precision%29) (TriggeredSeconds :type Float%20%28double-precision%29) (InputAction :type Input%20Action%20Object%20Reference :default "/Game/Input/IA_Crouch.IA_Crouch"))
  ;[0.15 0.15 0.15 0.5] TryCrouch
  (:Started
    (if (Class|MyPlayer|CanProcessActionInput)
      (if (AI|Components|NavMovement|IsCrouching (Variables|Character|GetCharacterMovement))
        (Character|UnCrouch)
        (else
          (Character|Crouch))))))

(event Input|EnhancedActionEvents|EnhancedInputActionIA_Assassination
  (params (ActionValue :type Boolean) (ElapsedSeconds :type Float%20%28double-precision%29) (TriggeredSeconds :type Float%20%28double-precision%29) (InputAction :type Input%20Action%20Object%20Reference :default "/Game/Input/IA_Assassination.IA_Assassination"))
  ;[0.15 0.15 0.15 0.5] TryAssassination
  (:Started
    (bind _returnvalue (Class|MyPlayer|BeginAssassionation))
    (if _returnvalue
      (bind _asbp_my_enemy (Utilities|Casting|CastToBP_MyEnemy (Variables|Default|GetEnemy)))
      (Class|MotionWarpingComponent|AddorUpdateWarpTargetfromLocationandRotation (Variables|Default|GetMotionWarping) "AssassinationTarget" (Transformation|GetWorldLocation (Variables|/Game/BluePrints/BP_MyEnemy.BP_MyEnemy_C|GetAssassinationPoint _asbp_my_enemy)) (Transformation|GetWorldRotation (Variables|/Game/BluePrints/BP_MyEnemy.BP_MyEnemy_C|GetAssassinationPoint _asbp_my_enemy)))
      (Animation|Montage|PlayMontage (Variables|Character|GetMesh) "/Game/Animations/Montages/AM_Assassination.AM_Assassination"
        (:then
          (Default|PlayChoke _asbp_my_enemy))
        (:OnCompleted
          (Class|MyPlayer|EndAssassionation))
        (:OnInterrupted
          (Class|MyPlayer|EndAssassionation))))))

(fn ConstructionScript)
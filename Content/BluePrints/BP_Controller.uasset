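; Player controller Blueprint that routes Enhanced Input to the controlled pawn for movement, camera look and rolling.
; On BeginPlay it adds the IMC_Player mapping context for the local controller.
; Move input drives the pawn along yaw-only forward and right vectors from the control rotation, while look input adds yaw and pitch.
; Roll input casts the pawn to BP_MyPlayer and calls TryRoll.
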(event Input|EnhancedActionEvents|EnhancedInputActionIA_Move
  (params (ActionValue :type Vector%202D%20Structure) (ElapsedSeconds :type Float%20%28double-precision%29) (TriggeredSeconds :type Float%20%28double-precision%29) (InputAction :type Input%20Action%20Object%20Reference :default "/Game/Input/IA_Move.IA_Move"))
  (bind _self self)
  (bind _self_2 self)
  (bind _returnvalue (Pawn|GetControlledPawn _self))
  (bind _returnvalue_2 (Pawn|GetControlRotation _self_2 :!class /Script/Engine.Controller))
  (bind _yaw (Math|Rotator|BreakRotator _returnvalue_2))
  (bind _returnvalue_3 (Math|Rotator|MakeRotator 0.0 0.0 _yaw))
  ;[0.15 0.15 0.15 0.5] WASD Move
  (bind _output_get (Variables|Default|SetMove%20Value ActionValue))
  (Pawn|Input|AddMovementInput _returnvalue (Math|Vector|GetRightVector _returnvalue_3) (.X (Math|Vector2D|BreakVector2D _output_get)) false)
  (Pawn|Input|AddMovementInput _returnvalue (Math|Vector|GetForwardVector _returnvalue_3) (.Y (Math|Vector2D|BreakVector2D _output_get)) false))

(event Input|EnhancedActionEvents|EnhancedInputActionIA_Look
  (params (ActionValue :type Vector%202D%20Structure) (ElapsedSeconds :type Float%20%28double-precision%29) (TriggeredSeconds :type Float%20%28double-precision%29) (InputAction :type Input%20Action%20Object%20Reference :default "/Game/Input/IA_Look.IA_Look"))
  (bind (_x _y) (Math|Vector2D|BreakVector2D ActionValue))
  ;[0.15 0.15 0.15 0.5] Mouse XY
  (Class|PlayerController|AddYawInput self _x)
  (Class|PlayerController|AddPitchInput self _y))

(event Input|EnhancedActionEvents|EnhancedInputActionIA_Roll
  (params (ActionValue :type Boolean) (ElapsedSeconds :type Float%20%28double-precision%29) (TriggeredSeconds :type Float%20%28double-precision%29) (InputAction :type Input%20Action%20Object%20Reference :default "/Game/Input/IA_Roll.IA_Roll"))
  ;[0.15 0.15 0.15 0.5] TryRoll
  (bind _asbp_my_player (Utilities|Casting|CastToBP_MyPlayer (Pawn|GetControlledPawn)))
  (Default|TryRoll _asbp_my_player))

(event EventBeginPlay
  ;[0.15 0.15 0.15 0.5] Controller
  (if (Pawn|IsLocalController self)
    (Input|AddMappingContext (PlayerController|LocalPlayerSubsystems|GetEnhancedInputLocalPlayerSubsystem self) "/Game/Input/IMC_Player.IMC_Player" 0 "(bIgnoreAllPressedKeysUntilRelease=True,bForceImmediately=False,bNotifyUserSettings=False)")))

(fn ConstructionScript)